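; Behavior tree node for guard AI that detects a player, though its detection logic is disconnected from the empty Tick and never runs.
; That logic sphere-traces around the guard, line-traces forward to confirm sight, and writes or clears the blackboard target.
; Sighting starts or resumes a timer calling FindPlayer, which sends InteractedMessage to the target.
; Losing sight pauses the timer, then clears it after a short delay.
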(event Custom|Player%20in%20sight
  ;[1 1 1] Starts the Timer
  (bind _returnvalue (Utilities|Time|SetTimerbyFunctionName self "FindPlayer" 4.0))
  (Development|PrintString "I see you" true true "(R=0.000000,G=0.660000,B=1.000000,A=1.000000)" 1.0))

(event Custom|Player%20not%20in%20sight
  ;[1 1 1] Clears the Timer
  (Utilities|Time|PauseTimerbyHandle (stale Custom|Player%20in%20sight _returnvalue))
  (Utilities|FlowControl|Delay 2.5)
  (Class|KismetSystemLibrary|ClearTimerHandle (stale Custom|Player%20in%20sight _returnvalue))
  (Development|PrintString "now i dont" true true "(R=0.000000,G=0.660000,B=1.000000,A=1.000000)" 1.0))

(event EventTick
  (params (OwnerActor :type Actor%20Object%20Reference) (DeltaSeconds :type Float%20%28single-precision%29))
  ;[1 1 1] IS the player inside the sphere
)

(fn FindPlayer
  (bind _playertarget (Variables|Default|GetPlayerTarget))
  (if (!= _playertarget 0)
    (Class|BPIInteractable|Interacted(Message) _playertarget false 0 false false)))
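; Ground spear trap that thrusts five spike meshes upward when an actor overlaps its trigger.
; After a configurable delay it offsets the meshes up, messages the stored target as a trap hit and plays a sound, then lowers them a second later.
; A TrapOn flag blocks retriggering, and leaving the trigger clears the target.
; Direct hits on any spike also send InteractedMessage to the other actor.
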(event OnComponentHit(StaticMesh)
  (params (OtherActor :type Actor%20Object%20Reference) (OtherComp :type Primitive%20Component%20Object%20Reference) (NormalImpulse :type Vector :default "0, 0, 0") (Hit :type Hit%20Result%20Structure%20%28by%20ref%29))
  (Class|BPIInteractable|Interacted(Message) OtherActor false 0 false false))

(event OnComponentHit(StaticMesh1)
  (params (OtherActor :type Actor%20Object%20Reference) (OtherComp :type Primitive%20Component%20Object%20Reference) (NormalImpulse :type Vector :default "0, 0, 0") (Hit :type Hit%20Result%20Structure%20%28by%20ref%29))
  (Class|BPIInteractable|Interacted(Message) OtherActor false 0 false false))

(event OnComponentHit(StaticMesh2)
  (params (OtherActor :type Actor%20Object%20Reference) (OtherComp :type Primitive%20Component%20Object%20Reference) (NormalImpulse :type Vector :default "0, 0, 0") (Hit :type Hit%20Result%20Structure%20%28by%20ref%29))
  (Class|BPIInteractable|Interacted(Message) OtherActor false 0 false false))

(event OnComponentHit(StaticMesh3)
  (params (OtherActor :type Actor%20Object%20Reference) (OtherComp :type Primitive%20Component%20Object%20Reference) (NormalImpulse :type Vector :default "0, 0, 0") (Hit :type Hit%20Result%20Structure%20%28by%20ref%29))
  (Class|BPIInteractable|Interacted(Message) OtherActor false 0 false false))

(event OnComponentHit(StaticMesh4)
  (params (OtherActor :type Actor%20Object%20Reference) (OtherComp :type Primitive%20Component%20Object%20Reference) (NormalImpulse :type Vector :default "0, 0, 0") (Hit :type Hit%20Result%20Structure%20%28by%20ref%29))
  (Class|BPIInteractable|Interacted(Message) OtherActor false 0 false false))

(event OnComponentBeginOverlap(Trigger)
  (params (OtherActor :type Actor%20Object%20Reference) (OtherComp :type Primitive%20Component%20Object%20Reference) (OtherBodyIndex :type Integer) (bFromSweep :type Boolean) (SweepResult :type Hit%20Result%20Structure%20%28by%20ref%29))
  (if (not (Variables|Default|GetTrapOn))
    (Variables|Default|SetTrapOn true)
    (Variables|Default|SetTarget OtherActor)
    (Utilities|FlowControl|Delay (Variables|Default|GetDelay%20Time%20on%20spikes))
    (Transformation|AddLocalOffset (Variables|Default|GetStaticMesh1) "0, 0,120.000000" false false)
    (Class|BPIInteractable|Interacted(Message) (Variables|Default|GetTarget) false 0 true false)
    ;[1 1 1] Added sound - joffre
    (Audio|PlaySound2D "/Game/Sounds/VariousSounds/Floor_spike_3.Floor_spike_3")
    (Utilities|FlowControl|Delay 1.0)
    (Transformation|AddLocalOffset (Variables|Default|GetStaticMesh1) "0, 0,-120.000000" false false)
    (Variables|Default|SetTrapOn false)))

(event OnComponentEndOverlap(Trigger)
  (params (OtherActor :type Actor%20Object%20Reference) (OtherComp :type Primitive%20Component%20Object%20Reference) (OtherBodyIndex :type Integer))
  (Variables|Default|SetTarget 0))

(event EventBeginPlay)

(event EventActorBeginOverlap
  (params (OtherActor :type Actor%20Object%20Reference)))

(event EventTick
  (params (DeltaSeconds :type Float%20%28single-precision%29)))

(fn ConstructionScript)
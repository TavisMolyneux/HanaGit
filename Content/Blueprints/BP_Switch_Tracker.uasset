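; BP_Switch_Tracker is an interactable switch that starts or stops a platform by setting its PlatformCanMove flag.
; InteractFunction calls OnInteract, which uses CanSwitch as a guard and branches on SwitchStatus to rotate the switch object and stop or start the platform.
; Starting requires RequirementFufilled, otherwise the switch rotates forward and straight back.
; SwitchStatus is never updated here, Interacted only returns false, and a debug print remains.
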(event EventBeginPlay)

(event EventActorBeginOverlap
  (params (OtherActor :type Actor%20Object%20Reference)))

(event EventTick
  (params (DeltaSeconds :type Float%20%28single-precision%29)))

(fn ConstructionScript)

(fn StartFunction
  (params (NewParam :type Simple%20Platform%20BP%20Object%20Reference))
  (Variables|/Game/SimplePlatform_BP.SimplePlatform_BP_C|SetPlatformCanMove NewParam true))

(fn StopFunction
  (params (NewParam :type Simple%20Platform%20BP%20Object%20Reference))
  (Variables|/Game/SimplePlatform_BP.SimplePlatform_BP_C|SetPlatformCanMove NewParam false))

(fn InteractFunction
  (CallFunction|OnInteract))

(fn OnInteract
  (Development|PrintString "aadfgsadfgo")
  (if (Variables|Default|GetCanSwitch)
    (Variables|Default|SetCanSwitch false)
    (if (Variables|Default|GetSwitchStatus)
      (Transformation|AddWorldRotation (Variables|Default|GetSwitch_Object) "0, 0,-90.000000" false false)
      (CallFunction|StopFunction (Variables|Default|GetPlatform))
      (Variables|Default|SetCanSwitch true)
      (elif (Variables|Default|GetRequirementFufilled)
        (Transformation|AddWorldRotation (Variables|Default|GetSwitch_Object) "0, 0,90.000000" false false)
        (CallFunction|StartFunction (Variables|Default|GetPlatform))
        (Variables|Default|SetCanSwitch true)
        (else
          (Transformation|AddWorldRotation (Variables|Default|GetSwitch_Object) "0, 0,90.000000" false false)
          (Transformation|AddWorldRotation (Variables|Default|GetSwitch_Object) "0, 0,-90.000000" false false)
          (Variables|Default|SetCanSwitch true)))))
  (return))

(fn Interacted
  (params (InteractInput :type Boolean) (NumberParam :type Integer))
  (return false))
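; BP_SwitchLevel1 is a switch-driven actor that lowers by MoveDistance from its starting height while active and rises back when inactive.
; Interacted sets CanMove from its Caught input, and Tick plays or reverses a timeline accordingly.
; The timeline's PlatformMove track lerps the Z position, and a DoOnce with no reset plays a 2D sound once it reaches a small threshold.
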(event EventBeginPlay
  (Variables|Default|SetStartZ (.Z (Math|Vector|BreakVector (Transformation|GetActorLocation)))))

(event EventActorBeginOverlap
  (params (OtherActor :type Actor%20Object%20Reference)))

(event EventTick
  (params (DeltaSeconds :type Float%20%28single-precision%29))
  (bind _returnvalue (Transformation|GetActorLocation))
  (bind (_x _y _z) (Math|Vector|BreakVector _returnvalue))
  (if (Variables|Default|GetCanMove)
    (bind _platformmove (Timeline|Timeline_0 Play)
      (:Update
        (Transformation|SetActorLocation (Math|Vector|MakeVector _x _y (Math|Float|Lerp (Variables|Default|GetStartZ) (- (Variables|Default|GetStartZ) (Variables|Default|GetMoveDistance)) _platformmove)) false false)
        (if (>= _platformmove 0.1)
          (Utilities|FlowControl|DoOnce false
            (:Completed
              (Audio|PlaySound2D (Variables|Default|GetSoundToPlay)))))))
    (else
      (Timeline|Timeline_0 Reverse))))

(fn ConstructionScript)

(fn Interacted
  (params (Caught :type Boolean) (NumberParam :type Integer) (Trap :type Boolean) (Falling :type Boolean))
  (Variables|Default|SetCanMove Caught)
  (return false))
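; BP_Dart is a dart projectile that flies in a straight line and self-destructs after a set lifespan.
; The construction script pitches the mesh 90 degrees, and Tick moves it along local Z by a per-frame speed, negated unless FacingRight.
; Hit and overlap send InteractedMessage to Player or Ignore-tagged actors, with overlap flagging it as a trap.
; The dart destroys itself on contact except with non-Player Ignore actors.
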(event OnComponentHit(StaticMeshComponent)
  (params (OtherActor :type Actor%20Object%20Reference) (OtherComp :type Primitive%20Component%20Object%20Reference) (NormalImpulse :type Vector :default "0, 0, 0") (Hit :type Hit%20Result%20Structure%20%28by%20ref%29))
  (bind _returnvalue (Actor|ActorHasTag OtherActor "Player"))
  ;[1 1 1] On Hit
  (if (or (Actor|ActorHasTag OtherActor "Ignore") _returnvalue)
    (Class|BPIInteractable|Interacted(Message) OtherActor false 0 false false)
    (if _returnvalue
      (Actor|DestroyActor :!label _label))
    (else
      (goto _label))))

(event OnComponentBeginOverlap(StaticMeshComponent)
  (params (OtherActor :type Actor%20Object%20Reference) (OtherComp :type Primitive%20Component%20Object%20Reference) (OtherBodyIndex :type Integer) (bFromSweep :type Boolean) (SweepResult :type Hit%20Result%20Structure%20%28by%20ref%29))
  (bind _returnvalue (Actor|ActorHasTag OtherActor "Player"))
  ;[1 1 1] On Overlap
  (if (or (Actor|ActorHasTag OtherActor "Ignore") _returnvalue)
    (Class|BPIInteractable|Interacted(Message) OtherActor false 0 true false)
    (if _returnvalue
      (Actor|DestroyActor :!label _label))
    (else
      (goto _label))))

(event EventBeginPlay
  ;[1 1 1] Dart speed, direction and lifespan
  (if (Variables|Default|GetFacing%20Right)
    _
    (else
      (Variables|Default|SetDart_Speed (* (Variables|Default|GetDart_Speed) -1.0))))
  (Utilities|FlowControl|Delay (Variables|Default|GetDart%20Life))
  (Actor|DestroyActor))

(event EventActorBeginOverlap
  (params (OtherActor :type Actor%20Object%20Reference)))

(event EventTick
  (params (DeltaSeconds :type Float%20%28single-precision%29))
  ;[1 1 1] Dart Movement
  (Transformation|AddLocalOffset (Variables|Debug|GetStaticMeshComponent) (Math|Vector|MakeVector 0.0 0.0 (Variables|Default|GetDart_Speed)) false false))

(fn ConstructionScript
  (Transformation|SetWorldRotation (Variables|Debug|GetStaticMeshComponent) "0, 0,90.000000" false false))
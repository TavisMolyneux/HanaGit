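; BP_Masher is a looping smasher hazard that moves a block vertically on a timed cycle.
; A wait timeline, started at 5 minus SmashTime, triggers the Smasher timeline, which lerps the block between its start point and CrusherLength below, then restarts the wait.
; Block hits send an Interacted message to the other actor.
; The construction script displays SmashTime on a text render.
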(event OnComponentHit(SmasherBlock)
  (params (OtherActor :type Actor%20Object%20Reference) (OtherComp :type Primitive%20Component%20Object%20Reference) (NormalImpulse :type Vector :default "0, 0, 0") (Hit :type Hit%20Result%20Structure%20%28by%20ref%29))
  (Class|BPIInteractable|Interacted(Message) OtherActor false))

(event EventBeginPlay
  (bind _smashtime (Variables|Default|GetSmashTime))
  (bind _returnvalue (- 5.0 _smashtime))
  ;[1 1 1] Smash Movement
  (Variables|Default|SetStartPoint (Transformation|GetWorldLocation (Variables|Default|GetSmasherBlock)))
  (Components|Timeline|SetPlaybackPosition (Variables|Default|GetTimeline_0) _returnvalue false true)
  (Timeline|Timeline_0 Play
    (:Finished
      (bind _newtrack_0 (Timeline|Smasher PlayFromStart)
        (:Update
          (Transformation|SetWorldLocation (Variables|Default|GetSmasherBlock) (Math|Vector|Lerp(Vector) (Variables|Default|GetStartPoint) (Math|Vector|MakeVector (.X (Math|Vector|BreakVector (Variables|Default|GetStartPoint))) (.Y (Math|Vector|BreakVector (Variables|Default|GetStartPoint))) (- (.Z (Math|Vector|BreakVector (Variables|Default|GetStartPoint))) (Variables|Default|GetCrusherLength))) _newtrack_0) false false))
        (:Finished
          (Components|Timeline|SetPlaybackPosition (Variables|Default|GetTimeline_0) _returnvalue false true)
          (Timeline|Timeline_0 Play))))))

(event EventActorBeginOverlap
  (params (OtherActor :type Actor%20Object%20Reference)))

(event EventTick
  (params (DeltaSeconds :type Float%20%28single-precision%29)))

(fn ConstructionScript
  (Rendering|Components|TextRender|SetText (Variables|Default|GetTextRender) (Utilities|Text|ToText(Float) (Variables|Default|GetSmashTime) "HalfToEven")))

(fn Interacted
  (params (InteractInput :type Boolean) (NumberParam :type Integer))
  (return false))
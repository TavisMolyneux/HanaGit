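; Guard AI character that patrols between two points, chases the player on detection and reports a catch when its capsule hits them.
; A FlipFlop alternates AIMoveTo patrol targets, with a short pause before each recursive Patrol call.
; DetectionBox overlaps toggle HasTarget, starting the chase and playing a spotted sound.
; A failed chase plays a fail sound and resumes patrol, but only if neither sound is already playing.
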(event OnComponentHit(CapsuleComponent)
  (params (OtherActor :type Actor%20Object%20Reference) (OtherComp :type Primitive%20Component%20Object%20Reference) (NormalImpulse :type Vector :default "0, 0, 0") (Hit :type Hit%20Result%20Structure%20%28by%20ref%29))
  (if (== OtherActor (Game|GetPlayerCharacter 0))
    (Class|BPIInteractable|Interacted(Message) OtherActor true 0 false false)))

(event OnComponentBeginOverlap(DetectionBox)
  (params (OtherActor :type Actor%20Object%20Reference) (OtherComp :type Primitive%20Component%20Object%20Reference) (OtherBodyIndex :type Integer) (bFromSweep :type Boolean) (SweepResult :type Hit%20Result%20Structure%20%28by%20ref%29))
  (if (== OtherActor (Game|GetPlayerCharacter 0))
    (Variables|Default|SetHasTarget true)
    (Variables|Default|SetPlayerTarget OtherActor)
    (CallFunction|MovetoPlayer)
    (if (not (Audio|Components|Audio|IsPlaying (Variables|Default|GetGuard_3_SpotFail)))
      (Audio|Components|Audio|Play (Variables|Default|GetGuard_3_Spotted) 0.0)
      (Development|PrintString "Hello"))))

(event OnComponentEndOverlap(DetectionBox)
  (params (OtherActor :type Actor%20Object%20Reference) (OtherComp :type Primitive%20Component%20Object%20Reference) (OtherBodyIndex :type Integer))
  (if (== OtherActor (Game|GetPlayerCharacter 0))
    (Variables|Default|SetHasTarget false)))

(event Custom|Patrol
  (if (not (Variables|Default|GetHasTarget))
    (Utilities|FlowControl|FlipFlop
      (:A
        (AI|AIMoveTo self "0, 0, 0" (Variables|Default|GetPatrolPoint1) 5.0 false
          (:OnSuccess
            (Utilities|FlowControl|Delay 2.0)
            (CallFunction|Patrol))))
      (:B
        (AI|AIMoveTo self "0, 0, 0" (Variables|Default|GetPatrolPoint2) 5.0 false
          (:OnSuccess
            (Utilities|FlowControl|Delay 2.0)
            (CallFunction|Patrol)))))))

(event Custom|MoveToPlayer
  (if (Variables|Default|GetHasTarget)
    (AI|AIMoveTo self "0, 0, 0" (Variables|Default|GetPlayerTarget) 5.0 false
      (:OnSuccess
        (Utilities|FlowControl|Delay 2.0 :!label _label)
        (CallFunction|Patrol))
      (:OnFail
        (if (not (or (Audio|Components|Audio|IsPlaying (Variables|Default|GetGuard_3_Spotted)) (Audio|Components|Audio|IsPlaying (Variables|Default|GetGuard_3_SpotFail))))
          (Audio|Components|Audio|Play (Variables|Default|GetGuard_3_SpotFail) 0.0)
          (Development|PrintString "Hello" true true "(R=1.000000,G=0.104356,B=0.037451,A=1.000000)")
          (goto _label))))))

(event EventBeginPlay
  (CallFunction|Patrol))

(event EventActorBeginOverlap
  (params (OtherActor :type Actor%20Object%20Reference)))

(event EventTick
  (params (DeltaSeconds :type Float%20%28single-precision%29))
  (if (Variables|Default|GetHasTarget)
    (Variables|Default|SetTargetDestination "0, 0, 0")))

(fn ConstructionScript)
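; BP_Switch is an interactable switch that relays interaction to a target object.
; BeginPlay caches the Switch component's relative location as its rest position.
; Interacted shifts the component slightly along negative local X when SwitchRequirementsMet is true, otherwise restores rest, then calls InteractedMessage on SwitchTarget either way and returns false.
; Tick checks the same flag but does nothing, and the interaction parameters go unused.
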(event EventBeginPlay
  (Variables|Default|SetStartLocation (Variables|/Script/Engine.SceneComponent|GetRelativeLocation (Variables|Default|GetSwitch))))

(event EventActorBeginOverlap
  (params (OtherActor :type Actor%20Object%20Reference)))

(event EventTick
  (params (DeltaSeconds :type Float%20%28single-precision%29))
  (if (Variables|Default|GetSwitchRequirementsMet)
    _))

(fn ConstructionScript)

(fn Interacted
  (params (Caught :type Boolean) (NumberParam :type Integer) (Trap :type Boolean) (Falling :type Boolean))
  (bind _startlocation (Variables|Default|GetStartLocation))
  (bind _switch (Variables|Default|GetSwitch))
  (bind (_x _y _z) (Math|Vector|BreakVector _startlocation))
  (if (Variables|Default|GetSwitchRequirementsMet)
    (Transformation|SetRelativeLocation _switch (Math|Vector|MakeVector (+ _x -5.0) _y _z) false false)
    (else
      (Transformation|SetRelativeLocation _switch (Variables|Default|GetStartLocation) false false)))
  (Class|BPIInteractable|Interacted(Message) (Variables|Default|GetSwitchTarget) false 0 false false)
  (return false))
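; BP_Dart_Trap_Statue is a statue trap that repeatedly fires BP_Dart projectiles from a spawn point with an attenuated sound.
; A Box overlap with a Player-tagged actor sets TargetFound and starts firing, while ContstantFire starts it on BeginPlay.
; A Delay of Cooldown loops the shot while either flag is true.
; End overlap is empty and the TargetFound reset is disconnected, so triggered firing never stops.
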(event OnComponentBeginOverlap(Box)
  (params (OtherActor :type Actor%20Object%20Reference) (OtherComp :type Primitive%20Component%20Object%20Reference) (OtherBodyIndex :type Integer) (bFromSweep :type Boolean) (SweepResult :type Hit%20Result%20Structure%20%28by%20ref%29))
  (if (Actor|ActorHasTag OtherActor "Player")
    (Variables|Default|SetTargetFound true)
    (CallFunction|CustomEvent0)))

(event OnComponentEndOverlap(Box)
  (params (OtherActor :type Actor%20Object%20Reference) (OtherComp :type Primitive%20Component%20Object%20Reference) (OtherBodyIndex :type Integer)))

(event Custom|CustomEvent_0
  (Game|SpawnActorfromClass "/Game/Blueprints/BP_Dart.BP_Dart_C" (Math|Conversions|ToTransform(Vector) (Transformation|GetWorldLocation (Variables|Default|GetSpawnPoint))) "Undefined" 0 1e+01 (Variables|Default|GetDart%20Lifespan) (Variables|Default|GetFacing%20right) :!label _label)
  (Audio|PlaySoundatLocation "/Game/Sounds/Dart_Cue.Dart_Cue" (Transformation|GetActorLocation) "0, 0, 0" 1.0 1.0 0.0 "/Game/Sounds/Dart_Attenuation.Dart_Attenuation")
  (Utilities|FlowControl|Delay (Variables|Default|GetCooldown))
  (if (or (Variables|Default|GetTargetFound) (Variables|Default|GetContstant%20fire))
    (goto _label)))

(event EventBeginPlay
  ;[1 1 1] If you want the delay to be scaled by cooldown, you can just plug cooldown into a delay node. otherwise just make the timeline 1 second and then use Cooldown to scale the play rate
  (if (Variables|Default|GetContstant%20fire)
    (Game|SpawnActorfromClass "/Game/Blueprints/BP_Dart.BP_Dart_C" (Math|Conversions|ToTransform(Vector) (Transformation|GetWorldLocation (Variables|Default|GetSpawnPoint))) "Undefined" 0 1e+01 (Variables|Default|GetDart%20Lifespan) (Variables|Default|GetFacing%20right) :!label _label)
    (Audio|PlaySoundatLocation "/Game/Sounds/Dart_Cue.Dart_Cue" (Transformation|GetActorLocation) "0, 0, 0" 1.0 1.0 0.0 "/Game/Sounds/Dart_Attenuation.Dart_Attenuation")
    (Utilities|FlowControl|Delay (Variables|Default|GetCooldown))
    (if (or (Variables|Default|GetTargetFound) (Variables|Default|GetContstant%20fire))
      (goto _label))))

(event EventActorBeginOverlap
  (params (OtherActor :type Actor%20Object%20Reference)))

(event EventTick
  (params (DeltaSeconds :type Float%20%28single-precision%29)))

(fn ConstructionScript)
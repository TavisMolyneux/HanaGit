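; BP_ConveyorBelt is a conveyor belt actor that carries side-scroller characters standing in its trigger box.
; Every Tick it offsets each overlapping SideScrollerCharacterUSETHIS along the belt's right vector, scaled by Speed and delta time, without sweep.
; The construction script inversely scales the Arrow component so it keeps its size when the belt is scaled.
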(event EventBeginPlay
  (Variables|Default|SetPlayerOnBelt false))

(event EventActorBeginOverlap
  (params (OtherActor :type Actor%20Object%20Reference)))

(event EventTick
  (params (DeltaSeconds :type Float%20%28single-precision%29))
  (for _array_element (Collision|GetOverlappingActors (Variables|Default|GetTriggerBox) "/Game/Blueprints/SideScrollerCharacterUSETHIS.SideScrollerCharacterUSETHIS_C" :!class /Script/Engine.PrimitiveComponent)
    (Transformation|AddActorWorldOffset _array_element (* (Math|Vector|GetRightVector (Transformation|GetActorRotation)) (* DeltaSeconds (Variables|Default|GetSpeed))))))

(fn ConstructionScript
  (Transformation|SetRelativeScale3D (Variables|Default|GetArrow) (/ "1.000000,1.000000,1.000000" (Transformation|GetActorScale3D))))
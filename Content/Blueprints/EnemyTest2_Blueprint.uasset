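; Test patrolling enemy that spots pawns ahead with a line trace and advances along its facing when alerted.
; A clamped sight timer scrubs a timeline driving the alert indicator's size, height and colour; filling it only prints a placeholder message.
; Overlaps flip idle patrol direction or, with a target, halt movement.
; StopBox volumes also set NoEdge, which blocks alerted advance and enables returning to spawn once sight is lost.
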(event OnComponentBeginOverlap(StaticMeshComponent)
  (params (OtherActor :type Actor%20Object%20Reference) (OtherComp :type Primitive%20Component%20Object%20Reference) (OtherBodyIndex :type Integer) (bFromSweep :type Boolean) (SweepResult :type Hit%20Result%20Structure%20%28by%20ref%29))
  (bind _currenttarget (Variables|Default|GetCurrentTarget))
  (bind _returnvalue (== _currenttarget 0))
  (if (Components|ComponentHasTag OtherComp "TurnAround")
    (if (Variables|Default|GetIdle) :!label _label
      (Transformation|AddWorldRotation (Variables|Debug|GetStaticMeshComponent) "0,180.000000,0.000000" false false :!label _label_2)
      (Variables|Default|SetCanMove true)
      (if (Variables|Default|GetFacingRight)
        (Variables|Default|SetFacingRight false)
        (else
          (Variables|Default|SetFacingRight true)))
      (elif _returnvalue
        (Variables|Default|SetIdle true)
        (Variables|Default|SetCanMove true)
        (else
          (Variables|Default|SetCanMove false :!label _label_3))))
    (elif (Components|ComponentHasTag OtherComp "StopBox")
      (Variables|Default|SetNoEdge true)
      (if _returnvalue
        (goto _label_2)
        (else
          (goto _label_3)))
      (else
        (goto _label)))))

(event OnComponentEndOverlap(StaticMeshComponent)
  (params (OtherActor :type Actor%20Object%20Reference) (OtherComp :type Primitive%20Component%20Object%20Reference) (OtherBodyIndex :type Integer))
  (if (Components|ComponentHasTag OtherComp "StopBox")
    (Variables|Default|SetNoEdge false)))

(event EventActorBeginOverlap
  (params (OtherActor :type Actor%20Object%20Reference)))

(event EventBeginPlay
  (Variables|Default|SetSpawnPos (Transformation|GetWorldLocation (Variables|Debug|GetStaticMeshComponent))))

(event EventTick
  (params (DeltaSeconds :type Float%20%28single-precision%29))
  (bind _speed (Variables|Default|GetSpeed))
  (bind _spawnpos (Variables|Default|GetSpawnPos))
  (bind _staticmeshcomponent (Variables|Debug|GetStaticMeshComponent))
  (bind _explinationimage_sprite (Variables|Default|GetExplinationImage_Sprite))
  (bind _explinationimage_sprite_2 (Variables|Default|GetExplinationImage_Sprite))
  (bind _staticmeshcomponent_2 (Variables|Debug|GetStaticMeshComponent))
  (bind _staticmeshcomponent_3 (Variables|Debug|GetStaticMeshComponent))
  (bind _returnvalue (Transformation|GetWorldLocation _staticmeshcomponent_2))
  (bind _returnvalue_2 (Transformation|GetRelativeTransform _explinationimage_sprite_2))
  (bind _returnvalue_3 (Math|Vector|MakeVector _speed 0.0 0.0))
  (bind _returnvalue_4 (Transformation|GetWorldLocation _staticmeshcomponent))
  (bind _location (Math|Transform|BreakTransform _returnvalue_2))
  (bind _returnvalue_5 (* _returnvalue_3 DeltaSeconds))
  (bind (_x _y) (Math|Vector|BreakVector _location))
  (Utilities|FlowControl|Sequence
    (:then_0
      ;[1 1 1] Spotting Player
      (Variables|Default|SetTimeSpottedTarget (Math|Float|Clamp(Float) (Variables|Default|GetTimeSpottedTarget) 0.0 5.0))
      (bind (_direction _size _position _colortest) (Timeline|SpottedTimeline SetNewTime)
        (:Update
          (Transformation|SetWorldScale3D (Variables|Default|GetAlert) (Math|Vector|MakeVector _size _size _size))
          (Transformation|SetRelativeLocation _explinationimage_sprite_2 (Math|Vector|MakeVector _x _y _position) false false)
          (Rendering|Material|SetVectorParameterValue (Variables|Default|GetSpottedDynamicMaterial) "SightedColour" _colortest :!class /Script/Engine.MaterialInstanceDynamic)
          (Sprite|SetSpriteColor _explinationimage_sprite_2 _colortest)
          (if (== (.X (Math|Vector|BreakVector (Transformation|GetWorldScale _explinationimage_sprite))) 0.01)
            (Development|SetHiddeninGame _explinationimage_sprite true false)
            (else
              (Development|SetHiddeninGame _explinationimage_sprite false false)))
          (bind (_outhit _returnvalue_6) (Collision|LineTraceForObjects _returnvalue (+ _returnvalue (* (Math|Vector|GetForwardVector (Transformation|GetWorldRotation _staticmeshcomponent_2)) (Variables|Default|GetSightDistance))) (Utilities|Array|MakeArray "ObjectTypeQuery3") false 0 "Persistent"))
          (if _returnvalue_6
            (bind _output_get (Variables|Default|SetTimeSpottedTarget (+ (* DeltaSeconds 1.0) (Variables|Default|GetTimeSpottedTarget))))
            (Variables|Default|SetCurrentTarget (.HitActor (Collision|BreakHitResult _outhit)))
            (Variables|Default|SetIdle false)
            (if (>= _output_get 5.0)
              (Variables|Default|SetTimeSpottedTarget 0.0)
              (Development|PrintString "Hello"))
            (else
              (Variables|Default|SetTimeSpottedTarget (- (Variables|Default|GetTimeSpottedTarget) (* DeltaSeconds 1.0)))
              (Variables|Default|SetCurrentTarget 0)
              (if (Variables|Default|GetNoEdge)
                (Variables|Default|SetReturnToStart true)))))))
    (:then_1
      (if (Variables|Default|GetCanMove)
        ;[1 1 1] Movment
        (if (Variables|Default|GetReturnToStart)
          (if (Variables|Default|GetIdle)
            (if (Variables|Default|GetIdle) :!label _label
              (if (Variables|Default|GetFacingRight)
                (Transformation|AddLocalOffset _staticmeshcomponent_3 _returnvalue_5 false false)
                (else
                  (Transformation|AddLocalOffset _staticmeshcomponent_3 (* (Math|Vector|MakeVector (* (Variables|Default|GetSpeed) -1.0) 0.0 0.0) DeltaSeconds) false false)))
              (elif (not (Variables|Default|GetNoEdge))
                (Transformation|AddLocalOffset _staticmeshcomponent_3 (* (Math|Vector|MakeVector (Variables|Default|GetSpeed) 0.0 0.0) DeltaSeconds) false false)))
            (else
              (Transformation|SetActorRotation (Math|Rotator|FindLookatRotation _returnvalue_4 _spawnpos))
              (Transformation|AddLocalOffset _staticmeshcomponent_3 _returnvalue_5 false false)
              (if (Math|Vector|Equal(Vector) _returnvalue_4 _spawnpos 1.0)
                (Variables|Default|SetReturnToStart false))))
          (else
            (goto _label)))))))

(fn ConstructionScript
  (bind _returnvalue (Rendering|Material|CreateDynamicMaterialInstance (Variables|Default|GetAlert) 0 0 :!class /Script/Engine.PrimitiveComponent))
  (Variables|Default|SetSpottedDynamicMaterial _returnvalue))
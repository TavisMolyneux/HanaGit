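; BP_Level2Door is a Level 2 door that opens once two switches are both activated.
; Its Interacted function sets the first or second switch flag from the number it receives and returns false.
; Tick checks both flags every frame, and when both are true it moves the actor 200 units above its BeginPlay location, hides the Cube mesh and disables collision.
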(event EventBeginPlay
  (Variables|Default|SetLocation (Transformation|GetActorLocation)))

(event EventActorBeginOverlap
  (params (OtherActor :type Actor%20Object%20Reference)))

(event EventTick
  (params (DeltaSeconds :type Float%20%28single-precision%29))
  (if (and (Variables|Default|GetSwitchOne) (Variables|Default|GetSwitchTwo))
    (Transformation|SetActorLocation (+ (Variables|Default|GetLocation) "0, 0,200.000000") false false)
    (Rendering|SetVisibility (Variables|Default|GetCube) false false)
    (Collision|SetActorEnableCollision false)))

(fn ConstructionScript)

(fn Interacted
  (params (Caught :type Boolean) (NumberParam :type Integer) (Trap :type Boolean) (Falling :type Boolean))
  (if (== NumberParam 1)
    (Variables|Default|SetSwitchOne true)
    (elif (== NumberParam 2)
      (Variables|Default|SetSwitchTwo true)))
  (return false))
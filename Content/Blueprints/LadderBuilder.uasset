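; LadderBuilder is a construction-time actor that builds a ladder from its origin to a LadderEnd vector.
; The construction script centers a Box component at half that vector and sets its Z extent to match.
; It derives the segment count from the vector's length and the mesh's Z bounds, then places evenly spaced, unrotated instances through an InstancedStaticMesh.
; The event graph has no active logic.
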(event EventBeginPlay)

(event EventActorBeginOverlap
  (params (OtherActor :type Actor%20Object%20Reference)))

(event EventTick
  (params (DeltaSeconds :type Float%20%28single-precision%29)))

(fn ConstructionScript
  (bind _instancedstaticmesh (Variables|Default|GetInstancedStaticMesh))
  (bind _box (Variables|Default|GetBox))
  (bind _ladderend (Variables|Default|GetLadderEnd))
  (bind _returnvalue (/ _ladderend 2))
  (bind _staticmesh (Variables|/Script/Engine.StaticMeshComponent|GetStaticMesh _instancedstaticmesh))
  (bind _boxextent (Variables|/Script/Engine.BoxComponent|GetBoxExtent _box))
  (bind _returnvalue_2 (StaticMesh|GetBoundingBox _staticmesh))
  (Components|Box|SetBoxExtent _box (Math|Vector|MakeVector (.x _boxextent) (.y _boxextent) (.Z (Math|Vector|BreakVector _returnvalue))) true)
  (Transformation|SetRelativeLocation _box _returnvalue false false)
  (Variables|Default|SetNumberOfLadders (Math|Float|Truncate (/ (Math|Vector|VectorLength (Variables|Default|GetLadderEnd)) (Math|Float|Max(Float) (Math|Float|Absolute(Float) (.z (.min _returnvalue_2))) (Math|Float|Absolute(Float) (.z (.max _returnvalue_2)))))))
  (LocalVariables|SetLadderSpacing (/ (Variables|Default|GetLadderEnd) (Variables|Default|GetNumberOfLadders)))
  (for _index (range 0 (Variables|Default|GetNumberOfLadders))
    (Components|InstancedStaticMesh|AddInstance (Variables|Default|GetInstancedStaticMesh) (Math|Transform|MakeTransform (LocalVariables|GetCurrentLadderLocation) "0, 0, 0" "1,1,1"))
    (LocalVariables|SetCurrentLadderLocation (* (LocalVariables|GetLadderSpacing) _index))))
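; BP_Trap_01 is a moving, rotating trap that notifies any actor it hits.
; Tick applies yaw rotation to the mesh and plays the Movement timeline, which lerps it from its BeginPlay location by MovementX and MovementY, keeping the starting height.
; A component hit sends the other actor an Interacted message flagged as Trap.
; The trap's own Interacted function is a stub returning false.
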(event OnComponentHit(StaticMeshComponent)
  (params (OtherActor :type Actor%20Object%20Reference) (OtherComp :type Primitive%20Component%20Object%20Reference) (NormalImpulse :type Vector :default "0, 0, 0") (Hit :type Hit%20Result%20Structure%20%28by%20ref%29))
  (Class|BPIInteractable|Interacted(Message) OtherActor false 0 true false))

(event EventBeginPlay
  (Variables|Default|SetStartLocation (Transformation|GetWorldLocation (Variables|Debug|GetStaticMeshComponent))))

(event EventActorBeginOverlap
  (params (OtherActor :type Actor%20Object%20Reference)))

(event EventTick
  (params (DeltaSeconds :type Float%20%28single-precision%29))
  (bind _startlocation (Variables|Default|GetStartLocation))
  (bind (_x _y _z) (Math|Vector|BreakVector _startlocation))
  (Transformation|AddLocalRotation (Variables|Debug|GetStaticMeshComponent) (Math|Rotator|MakeRotator 0.0 0.0 (Variables|Default|GetRotation_speed)) false false)
  ;[1 1 1] Instead of using Play Sound 2d, add a sound component and then use the reverse of your timeline to set the location of the sound component, that way even if the log moves, the sound will stay in the same location so the player can hear it.
  (bind _movement (Timeline|Movement Play)
    (:Update
      (Transformation|SetWorldLocation (Variables|Debug|GetStaticMeshComponent) (Math|Vector|Lerp(Vector) _startlocation (Math|Vector|MakeVector (+ _x (Variables|Default|GetMovement%20X)) (+ _y (Variables|Default|GetMovement%20Y)) _z) _movement) false false))))

(fn ConstructionScript)

(fn Interacted
  (params (Caught :type Boolean) (NumberParam :type Integer) (Trap :type Boolean) (Falling :type Boolean))
  (return false))
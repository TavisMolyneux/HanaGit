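; SimplePlatform_BP is a platform actor that moves between its starting position and a TargetLocation component's position captured at BeginPlay.
; Interacted sets PlatformCanMove from its input, and Tick plays or reverses UpmovementTimeline accordingly.
; The timeline lerps between the two cached points, applying the result as relative location without sweep.
; Tick also prints the movement alpha every frame for debugging.
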(event EventBeginPlay
  (Variables|Default|SetPlatformStartingPosition (Transformation|GetActorLocation))
  (Variables|Default|SetPlatformTargetLocation (Transformation|GetWorldLocation (Variables|Default|GetTargetLocation))))

(event EventActorBeginOverlap
  (params (OtherActor :type Actor%20Object%20Reference)))

(event EventTick
  (params (DeltaSeconds :type Float%20%28single-precision%29))
  (Development|PrintString (Utilities|String|ToString(Float) (Variables|Default|GetPlatformMovementAlpha)) true true "(R=0.000000,G=0.660000,B=1.000000,A=1.000000)" 0.0)
  (if (Variables|Default|GetPlatformCanMove)
    (bind _newtrack_2 (Timeline|UpmovementTimeline Play)
      (:Update
        (Variables|Default|SetPlatformMovementAlpha _newtrack_2)
        (Transformation|SetActorRelativeLocation (Math|Vector|Lerp(Vector) (Variables|Default|GetPlatformStartingPosition) (Variables|Default|GetPlatformTargetLocation) _newtrack_2))))
    (else
      (Timeline|UpmovementTimeline Reverse))))

(fn ConstructionScript)

(fn Interacted
  (params (InteractInput :type Boolean) (NumberParam :type Integer))
  (Variables|Default|SetPlatformCanMove InteractInput)
  (return false))